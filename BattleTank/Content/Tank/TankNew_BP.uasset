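; Player-controllable tank pawn Blueprint that wires input to aiming and movement components and sets up its health bar.
; On BeginPlay it initialises TankAiming with turret and barrel, TankMovement with both tracks, and passes itself to the HealthBar widget.
; Fire and drive inputs forward intents to those components, while aim axes rotate an azimuth gimbal and spring arm for the camera.
; Swap Camera toggles between first- and third-person cameras.
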(event EventBeginPlay
  (Class|TankAimingComponent|Initialise (Variables|Default|GetTankAiming) (Variables|Default|GetTankTurret) (Variables|Default|GetTankBarrel))
  (Class|TankMovementComponent|Initialise (Variables|Default|GetTankMovement) (Variables|Default|GetRightTrack) (Variables|Default|GetLeftTrack))
  (CallFunction|InitializeHealthBar))

(event Collision|EventActorBeginOverlap
  (params (OtherActor :type Actor%20Object%20Reference)))

(event EventTick
  (params (DeltaSeconds :type Float%20%28single-precision%29)))

(event Input|ActionEvents|InputActionSwapCamera
  (params (Key :type Key%20Structure))
  ;[1 1 1] Camera input binding
  (:Pressed
    (Components|Activation|ToggleActive (Variables|Default|Get1st%20Person))
    (Components|Activation|ToggleActive (Variables|Default|Get3rd%20Person))))

(event Input|ActionEvents|InputActionFire
  (params (Key :type Key%20Structure))
  ;[1 1 1] Gameplay input binding
  (:Pressed
    (Class|TankAimingComponent|Fire (Variables|Default|GetTankAiming))))

(event Input|AxisEvents|InputAxisAimAzimuth
  (params (AxisValue :type Float%20%28single-precision%29))
  ;[1 1 1] Camera input binding
  (Transformation|AddLocalRotation (Variables|Default|GetAzimuth%20Gimbal) (Math|Rotator|MakeRotator 0.0 0.0 AxisValue) false false))

(event Input|AxisEvents|InputAxisAimAltitude
  (params (AxisValue :type Float%20%28single-precision%29))
  ;[1 1 1] Camera input binding
  (Transformation|AddLocalRotation (Variables|Default|GetSpringArm) (Math|Rotator|MakeRotator 0.0 AxisValue 0.0) false false))

(event Input|AxisEvents|InputAxisMoveForward
  (params (AxisValue :type Float%20%28single-precision%29))
  ;[1 1 1] Gameplay input binding
  (Class|TankMovementComponent|IntendMoveForward (Variables|Default|GetTankMovement) AxisValue))

(event Input|AxisEvents|InputAxisRotateClockwise
  (params (AxisValue :type Float%20%28single-precision%29))
  ;[1 1 1] Gameplay input binding
  (Class|TankMovementComponent|IntendRotateClockwise (Variables|Default|GetTankMovement) AxisValue))

(fn ConstructionScript)

(fn InitializeHealthBar
  (bind _ashealth_bar (Utilities|Casting|CastToHealthBar (UserInterface|GetUserWidgetObject (Variables|Default|GetHealth))))
  (Variables|/Game/UI/HealthBar.HealthBar_C|SetMyTank _ashealth_bar self)
  (return))