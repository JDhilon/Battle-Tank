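; Player-controllable tank pawn Blueprint that wires up aiming, movement and firing.
; On BeginPlay it hands the turret and barrel to TankAiming and the two tracks to TankMovement.
; Movement axes pass forward and rotation intents to TankMovement, and the Fire action calls Fire.
; Camera axes rotate an azimuth gimbal for yaw and the spring arm for pitch, keeping the two rotations on separate components.
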(event EventBeginPlay
  (Class|TankAimingComponent|Initialise (Variables|Default|GetTankAiming) (Variables|Default|GetTankTurret) (Variables|Default|GetTankBarrel))
  (Class|TankMovementComponent|Initialise (Variables|Default|GetTankMovement) (Variables|Default|GetRightTrack) (Variables|Default|GetLeftTrack)))

(event Collision|EventActorBeginOverlap
  (params (OtherActor :type Actor%20Object%20Reference)))

(event EventTick
  (params (DeltaSeconds :type Float%20%28single-precision%29)))

(event Input|ActionEvents|InputActionFire
  (params (Key :type Key%20Structure))
  ;[1 1 1] Gameplay input binding
  (:Pressed
    (Class|Tank|Fire)))

(event Input|AxisEvents|InputAxisAimAzimuth
  (params (AxisValue :type Float%20%28single-precision%29))
  ;[1 1 1] Camera input binding
  (Transformation|AddLocalRotation (Variables|Default|GetAzimuthGimbal) (Math|Rotator|MakeRotator 0.0 0.0 AxisValue) false false))

(event Input|AxisEvents|InputAxisAimAltitude
  (params (AxisValue :type Float%20%28single-precision%29))
  ;[1 1 1] Camera input binding
  (Transformation|AddLocalRotation (Variables|Default|GetSpringArm) (Math|Rotator|MakeRotator 0.0 AxisValue 0.0) false false))

(event Input|AxisEvents|InputAxisMoveForward
  (params (AxisValue :type Float%20%28single-precision%29))
  ;[1 1 1] Gameplay input binding
  (Class|TankMovementComponent|IntendMoveForward (Variables|Default|GetTankMovement) AxisValue))

(event Input|AxisEvents|InputAxisRotateClockwise
  (params (AxisValue :type Float%20%28single-precision%29))
  ;[1 1 1] Gameplay input binding
  (Class|TankMovementComponent|IntendRotateClockwise (Variables|Default|GetTankMovement) AxisValue))

(fn ConstructionScript)